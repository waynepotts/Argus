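; Debug visual actor for an Argus entity, reflecting selection, faction, team, death and passenger state in the world.
; BeginPlay creates a dynamic material on the Cone, which team and death events recolor.
; Other events toggle the selection decal, hover overlay and actor visibility, or write the faction name to a text render.
; Waypoints and targets appear as brief debug capsules, while the under-attack event does nothing, leaving its print logic disconnected.
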(event `self.ReceiveBeginPlay`
  (bind _cone (`self.Cone`)
    (:`then`
      (bind _returnvalue (`PrimitiveComponent.CreateDynamicMaterialInstance` _cone 1 (`PrimitiveComponent.GetMaterial` _cone 1) "None"))
      (set `self.TeamColorMaterial` _returnvalue))
    (:`else`)))

(event `self.OnSelected`
  ;[1 0 0] Debug functionality
  (`self.OnSelected_BP`))

(event `self.OnDeselected`
  ;[1 0 0] Debug functionality
  (`self.OnDeselected_BP`))

(event `self.OnPopulateFaction`
  (params (factionRecord :type "FactionRecord Object Reference"))
  ;[1 0 0] Debug functionality
  (`self.OnPopulateFaction_BP` factionRecord))

(event `self.OnPopulateTeam`
  (params (teamColor :type "Color Structure"))
  ;[1 0 0] Debug functionality
  (`self.OnPopulateTeam_BP` teamColor))

(event `self.OnArgusEntityDeath`
  ;[1 0 0] Debug functionality
  (`self.OnArgusEntityDeath_BP`))

(event `self.OnArgusEntityPassengerStateChanged`
  (params (isPassenger :type Boolean))
  ;[1 0 0] Debug functionality
  (if isPassenger
    (`self.OnBecomePassenger_BP`)
    (else
      (`self.OnVacateCarrier_BP`)
      (`self.OnDeselected_BP`))))

(event `self.SetCurrentWaypointsVisible`
  (params (bVisible :type Boolean))
  (`parent.SetCurrentWaypointsVisible` bVisible)
  (if bVisible
    (for _array_element (`self.GetCurrentWaypoints`)
      (`KismetSystemLibrary.DrawDebugCapsule` _array_element 50.0 30.0 (struct) (struct :`R` 1.0 :`G` 1.0 :`B` 1.0 :`A` 1.0) 1.0 1.0))))

(event `self.SetCurrentTargetVisible`
  (params (bVisible :type Boolean))
  (bind _returnvalue (`self.GetCurrentTargetLocation`))
  (`parent.SetCurrentTargetVisible` bVisible)
  (if (and bVisible (!= _returnvalue (0.0 0.0 0.0) :`ErrorTolerance` 0.1))
    (`KismetSystemLibrary.DrawDebugCapsule` _returnvalue 50.0 30.0 (struct) (struct :`R` 0.040479 :`G` 1.0 :`B` 0.074658 :`A` 1.0) 1.0 1.0)))

(event `self.OnCursorHover`
  (params (bHover :type Boolean))
  (`MeshComponent.SetOverlayMaterial` (`self.Cone`) (select `bool` bHover :`true` "/Game/Art/Materials/OverlayMat_Inst.OverlayMat_Inst" :!type "MaterialInterface Object Reference")))

(event `self.ArgusEntityUnderAttack`)

(fn `OnArgusEntityDeath_BP`
  ;[1 0 0] Debug functionality
  (bind _teamcolormaterial (`self.TeamColorMaterial`)
    (:`then`
      (`MaterialInstanceDynamic.SetVectorParameterValue` _teamcolormaterial "Base Color" (struct :`R` 0.118056 :`G` 0.118056 :`B` 0.118056 :`A` 1.0)))
    (:`else`)))

(fn `OnBecomePassenger_BP`
  ;[1 0 0] Debug functionality
  (bind _rootcomponent (`self.RootComponent`)
    (:`then`
      (`SceneComponent.SetHiddenInGame` _rootcomponent true true))
    (:`else`)))

(fn `OnDeselected_BP`
  ;[1 0 0] Debug functionality
  (bind _selection_circle_decal (`self.Selection Circle Decal`)
    (:`then`
      (`SceneComponent.SetHiddenInGame` _selection_circle_decal true true))
    (:`else`)))

(fn `OnPopulateFaction_BP`
  (params (`Faction Record` :type "FactionRecord Object Reference"))
  ;[1 0 0] Debug functionality
  (bind _textrender (`self.TextRender`)
    (:`then`
      (bind _faction_record (`local.Faction Record`)
        (:`then`
          (`TextRenderComponent.K2_SetText` _textrender (`KismetTextLibrary.Conv_StringToText` (`FactionRecord.m_factionName` _faction_record))))
        (:`else`
          (`TextRenderComponent.K2_SetText` _textrender (`KismetTextLibrary.Conv_StringToText` "")))))
    (:`else`)))

(fn `OnPopulateTeam_BP`
  (params (`Team Color` :type "Color Structure"))
  ;[1 0 0] Debug functionality
  (bind _teamcolormaterial (`self.TeamColorMaterial`)
    (:`then`
      (`MaterialInstanceDynamic.SetVectorParameterValue` _teamcolormaterial "Base Color" (`KismetMathLibrary.Conv_ColorToLinearColor` `Team Color`)))
    (:`else`)))

(fn `OnSelected_BP`
  ;[1 0 0] Debug functionality
  (bind _selection_circle_decal (`self.Selection Circle Decal`)
    (:`then`
      (`SceneComponent.SetHiddenInGame` _selection_circle_decal false true))
    (:`else`)))

(fn `OnVacateCarrier_BP`
  ;[1 0 0] Debug functionality
  (bind _rootcomponent (`self.RootComponent`)
    (:`then`
      (`SceneComponent.SetHiddenInGame` _rootcomponent false true))
    (:`else`)))

(fn `UserConstructionScript`)