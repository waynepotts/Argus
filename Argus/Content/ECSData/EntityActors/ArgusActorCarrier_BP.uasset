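; Actor Blueprint for the Argus carrier entity, providing debug visuals for selection, faction, team and death.
; BeginPlay makes a dynamic material on the Cone, which is tinted to the team color and turns dark gray on death.
; Entity events forward to matching functions, which show the faction name on a text render and toggle selection indicators.
; Flying uses the SelectionCircle and grounded uses the decal, swapped on take-off and landing.
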(event `self.ReceiveBeginPlay`
  (bind _cone (`self.Cone`)
    (:`then`
      (bind _returnvalue (`PrimitiveComponent.CreateDynamicMaterialInstance` _cone 0 (`PrimitiveComponent.GetMaterial` _cone 0) "None"))
      (set `self.TeamColorMaterial` _returnvalue))
    (:`else`)))

(event `self.OnSelected`
  ;[1 0 0] Debug functionality
  (`self.OnSelected_BP`))

(event `self.OnDeselected`
  ;[1 0 0] Debug functionality
  (`self.OnDeselected_BP`))

(event `self.OnPopulateFaction`
  (params (factionRecord :type "FactionRecord Object Reference"))
  ;[1 0 0] Debug functionality
  (`self.OnPopulateFaction_BP` factionRecord))

(event `self.OnPopulateTeam`
  (params (teamColor :type "Color Structure"))
  ;[1 0 0] Debug functionality
  (`self.OnPopulateTeam_BP` teamColor))

(event `self.OnArgusEntityDeath`
  ;[1 0 0] Debug functionality
  (`self.OnArgusEntityDeath_BP`))

(event `self.OnTakeOff`
  ;[1 0 0] Debug functionality
  (`self.OnTakeOff_BP`))

(event `self.OnLand`
  ;[1 0 0] Debug functionality
  (`self.OnLand_BP`))

(fn `OnArgusEntityDeath_BP`
  ;[1 0 0] Debug functionality
  (bind _teamcolormaterial (`self.TeamColorMaterial`)
    (:`then`
      (`MaterialInstanceDynamic.SetVectorParameterValue` _teamcolormaterial "Base Color" (struct :`R` 0.118056 :`G` 0.118056 :`B` 0.118056 :`A` 1.0)))
    (:`else`)))

(fn `OnDeselected_BP`
  ;[1 0 0] Debug functionality
  (bind _selection_circle_decal (`self.Selection Circle Decal`)
    (:`then`
      (`SceneComponent.SetHiddenInGame` _selection_circle_decal true true))
    (:`else`
      _))
  (bind _selection_circle (`self.Selection Circle`)
    (:`then`
      (`SceneComponent.SetHiddenInGame` _selection_circle true true))
    (:`else`)))

(fn `OnLand_BP`
  ;[1 0 0] Debug functionality
  (bind _selection_circle_decal (`self.Selection Circle Decal`)
    (:`then`
      (`SceneComponent.SetHiddenInGame` _selection_circle_decal false true))
    (:`else`
      _))
  (bind _selection_circle (`self.Selection Circle`)
    (:`then`
      (`SceneComponent.SetHiddenInGame` _selection_circle true true))
    (:`else`)))

(fn `OnPopulateFaction_BP`
  (params (FactionRecord :type "FactionRecord Object Reference"))
  ;[1 0 0] Debug functionality
  (bind _textrender (`self.TextRender`)
    (:`then`
      (bind _factionrecord (`local.FactionRecord`)
        (:`then`
          (`TextRenderComponent.K2_SetText` _textrender (`KismetTextLibrary.Conv_StringToText` (`FactionRecord.m_factionName` _factionrecord))))
        (:`else`
          (`TextRenderComponent.K2_SetText` _textrender (`KismetTextLibrary.Conv_StringToText` "")))))
    (:`else`)))

(fn `OnPopulateTeam_BP`
  (params (TeamColor :type "Color Structure"))
  ;[1 0 0] Debug functionality
  (bind _teamcolormaterial (`self.TeamColorMaterial`)
    (:`then`
      (`MaterialInstanceDynamic.SetVectorParameterValue` _teamcolormaterial "Base Color" (`KismetMathLibrary.Conv_ColorToLinearColor` TeamColor)))
    (:`else`)))

(fn `OnSelected_BP`
  ;[1 0 0] Debug functionality
  (if (`self.IsFlying`)
    (bind _selection_circle_decal (`self.Selection Circle Decal`)
      (:`then`
        (`SceneComponent.SetHiddenInGame` _selection_circle_decal true true))
      (:`else`
        _))
    (bind _selection_circle (`self.Selection Circle`)
      (:`then`
        (`SceneComponent.SetHiddenInGame` _selection_circle false true))
      (:`else`))
    (else
      (bind _selection_circle_decal_2 (`self.Selection Circle Decal`)
        (:`then`
          (`SceneComponent.SetHiddenInGame` _selection_circle_decal_2 false true))
        (:`else`
          _))
      (bind _selection_circle_2 (`self.Selection Circle`)
        (:`then`
          (`SceneComponent.SetHiddenInGame` _selection_circle_2 true true))
        (:`else`)))))

(fn `OnTakeOff_BP`
  ;[1 0 0] Debug functionality
  (bind _selection_circle_decal (`self.Selection Circle Decal`)
    (:`then`
      (`SceneComponent.SetHiddenInGame` _selection_circle_decal true true))
    (:`else`
      _))
  (bind _selection_circle (`self.Selection Circle`)
    (:`then`
      (`SceneComponent.SetHiddenInGame` _selection_circle false true))
    (:`else`)))

(fn `UserConstructionScript`)